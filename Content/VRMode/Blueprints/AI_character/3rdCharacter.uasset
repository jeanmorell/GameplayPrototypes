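; 3rdCharacter is an AI-moved character for VR mode that walks to requested locations or actors.
; MoveTo sends it to a given location through AIMoveTo.
; MoveToSphere moves it toward the passed-in actor only when it is over 150 units from the TargetSphereActor found in the level.
; On BeginPlay it caches the player's VRPawn_OVR, though nothing here uses that reference.
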(event Custom|Move%20To
  (params (Location :type Vector))
  (AI|AIMoveTo self Location 0 5.0 true))

(event Custom|Move%20To%20Sphere
  (params (NewParam :type Actor%20Object%20Reference))
  (bind _returnvalue (Actor|GetActorOfClass "/Game/VRMode/Blueprints/TargetSphere/TargetSphereActor.TargetSphereActor_C"))
  (if (> (Transformation|GetDistanceTo _returnvalue) 1.5e+02)
    (AI|AIMoveTo self "0, 0, 0" NewParam 5.0 true)))

(event EventBeginPlay
  (bind _asvrpawn_ovr (Utilities|Casting|CastToVRPawn_OVR (Game|Player|GetPlayerPawn 0)))
  (Variables|Default|SetVRPawn _asvrpawn_ovr))

(fn ConstructionScript)
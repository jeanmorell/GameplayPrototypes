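; AI_Lutin is a flying imp in the VR mode that wanders and swaps paintings.
; CreateNewDestination picks either a random point on a fixed-X plane or a painting's position, re-rolling random indices per loop iteration to choose the pair.
; Tick moves it by constant-speed interpolation rather than AI navigation, choosing again after arrival.
; At a painting, it swaps both paintings' locations and CadreIDs unless the VR pawn has one selected.
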(event Custom|Create%20new%20destination
  (if (> (Math|Random|RandomFloat) 0.5)
    (Variables|Default|SetIsGoingToPainting true)
    (bind _outactors (Actor|GetAllActorsOfClass "/Game/VRMode/Blueprints/Interactables/Painting.Painting_C"))
    (for (_array_element _array_index) _outactors
      (if (== _array_index (Math|Random|RandomInteger (- (Utilities|Array|Length _outactors) 1)))
        (bind _output_get (Variables|Default|SetPainting%20destination _array_element))
        (Variables|Default|SetPainting%20Destination%20Location (Transformation|GetActorLocation _output_get))
        (Variables|Default|SetPainting%20Destination%20Cadre%20ID (Variables|/Game/VRMode/Blueprints/Interactables/Painting.Painting_C|GetCadre_ID _output_get)))
      (if (== _array_index (Math|Random|RandomInteger (- (Utilities|Array|Length _outactors) 1)))
        (bind _output_get_2 (Variables|Default|SetPainting%20Origin _array_element))
        (Variables|Default|SetPainting%20Origin%20location (Transformation|GetActorLocation _output_get_2))
        (Variables|Default|SetPainting%20Origin%20Cadre%20ID (Variables|/Game/VRMode/Blueprints/Interactables/Painting.Painting_C|GetCadre_ID _output_get_2))))
    (Development|PrintString (Utilities|String|ToString(Integer) (Math|Random|RandomInteger (- (Utilities|Array|Length _outactors) 1))))
    (Development|PrintString (Utilities|String|ToString(Integer) (Math|Random|RandomInteger (- (Utilities|Array|Length _outactors) 1))))
    (Variables|Default|SetDestination (Math|Vector|MakeVector -1.8e+02 (.y (Variables|Default|GetPainting%20Destination%20Location)) (.z (Variables|Default|GetPainting%20Destination%20Location))))
    (else
      (Variables|Default|SetDestination (Math|Vector|MakeVector -1.8e+02 (Math|Random|RandomFloatinRange -1.6e+02 1.9e+02) (Math|Random|RandomFloatinRange -1.8e+02 1.8e+02)))
      (Development|PrintString "new destination"))))

(event Custom|Flyinf
  (bind _self self)
  (bind _sphere (Variables|Default|GetSphere _self))
  (Transformation|SetWorldLocation _sphere (Math|Interpolation|VInterptoConstant (Transformation|GetWorldLocation _sphere) (Variables|Default|GetDestination) (stale EventTick DeltaSeconds) (Variables|Default|GetInterp%20Speed)) false false)
  (Transformation|SetActorLocation (Math|Interpolation|VInterptoConstant (Transformation|GetWorldLocation _sphere) (Variables|Default|GetDestination) (stale EventTick DeltaSeconds) (Variables|Default|GetInterp%20Speed)) false false))

(event Custom|Swap%20paintings
  (bind _asvrpawn_ha_s (Utilities|Casting|CastToVRPawn_HaS (Game|Player|GetPlayerPawn 0)))
  (if (not (Variables|/Game/VRMode/Blueprints/VRCamera/VRPawn_HaS.VRPawn_HaS_C|GetHasSelectedPainting _asvrpawn_ha_s))
    (Transformation|SetActorLocation (Variables|Default|GetPainting%20Origin) (Variables|Default|GetPainting%20Destination%20Location) false false)
    (Variables|/Game/VRMode/Blueprints/Interactables/Painting.Painting_C|SetCadre_ID (Variables|Default|GetPainting%20Origin) (Variables|Default|GetPainting%20Destination%20Cadre%20ID))
    (Transformation|SetActorLocation (Variables|Default|GetPainting%20destination) (Variables|Default|GetPainting%20Origin%20location) false false)
    (Variables|/Game/VRMode/Blueprints/Interactables/Painting.Painting_C|SetCadre_ID (Variables|Default|GetPainting%20destination) (Variables|Default|GetPainting%20Origin%20Cadre%20ID))
    (Development|PrintString "Paintings swapped !")))

(event EventBeginPlay
  (CallFunction|CreateNewDestination)
  (Utilities|FlowControl|Delay 1.0)
  (bind _outactors (Actor|GetAllActorsOfClass "/Game/VRMode/Blueprints/Assets/Cadre.Cadre_C"))
  (Variables|Default|SetCadres _outactors))

(event Collision|EventActorBeginOverlap
  (params (OtherActor :type Actor%20Object%20Reference)))

(event EventTick
  (params (DeltaSeconds :type Float%20%28single-precision%29))
  (if (< (Math|Vector|Distance(Vector) (Transformation|GetWorldLocation (Variables|Default|GetSphere)) (Variables|Default|GetDestination)) 0.2)
    (if (Variables|Default|GetIsGoingToPainting)
      (CallFunction|SwapPaintings)
      (Variables|Default|SetIsGoingToPainting false))
    (Utilities|FlowControl|Delay 1.0)
    (CallFunction|CreateNewDestination))
  (CallFunction|Flyinf))

(fn ConstructionScript)
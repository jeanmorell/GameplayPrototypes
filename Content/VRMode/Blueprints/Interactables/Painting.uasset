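; VR interactable painting that the player picks up and moves to another frame (Cadre), swapping places with the painting already there.
; Activation registers it on VRPawn_HaS and reveals the other frames; while selected, it follows the pawn's hit location in Y and Z.
; Deselection waits briefly, hides the frames, then swaps both paintings' locations and CadreIDs.
; A camera-facing CircleWidget displays interaction timing.
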(event EventOnFocus
  ;[1 1 1] Interface events
  (Development|PrintString "Focus"))

(event EventOnBlur
  ;[1 1 1] Interface events
  (Development|PrintString "BLUR" true true "(R=0.218356,G=1.000000,B=0.000000,A=1.000000)")
  (Utilities|Time|ClearandInvalidateTimerbyHandle (Variables|Default|GetInteraction%20Time))
  (Variables|Default|SetTime 0.0))

(event EventTick
  (params (DeltaSeconds :type Float%20%28single-precision%29))
  ;[1 1 1] Draw Circle logic
  (Transformation|SetWorldRotation (Variables|Default|GetCircleWidget) (Math|Rotator|FindLookatRotation (Transformation|GetWorldLocation (Variables|Default|GetCircleWidget)) (Transformation|GetWorldLocation (Variables|/Script/Engine.PlayerCameraManager|GetTransformComponent (Game|GetPlayerCameraManager 0)))) false false)
  (bind _focustime (CallFunction|GetFocusTime))
  (bind _ascircle_widget (Utilities|Casting|CastToCircleWidget (UserInterface|GetWidget (Variables|Default|GetCircleWidget))))
  (Variables|/Game/VRMode/Blueprints/Widgets/InteractionWidgets/CircleWidget.CircleWidget_C|SetTime _ascircle_widget _focustime)
  (Variables|/Game/VRMode/Blueprints/Widgets/InteractionWidgets/CircleWidget.CircleWidget_C|SetTimer _ascircle_widget (Variables|Default|GetInteraction%20Time))
  (if (Variables|Default|GetIsSelected)
    (bind _asvrpawn_ha_s (Utilities|Casting|CastToVRPawn_HaS (Game|Player|GetPlayerPawn 0)))
    (Transformation|SetActorLocation (Math|Vector|MakeVector (.x (Transformation|GetActorLocation self)) (.y (Variables|/Game/VRMode/Blueprints/VRCamera/VRPawn_HaS.VRPawn_HaS_C|GetHit%20Location _asvrpawn_ha_s)) (.z (Variables|/Game/VRMode/Blueprints/VRCamera/VRPawn_HaS.VRPawn_HaS_C|GetHit%20Location _asvrpawn_ha_s))) false false)))

(event EventOnActivate
  ;[1 1 1] Interface events
  (Development|PrintString "WTFFFFFFFFFFFFFFFFFFFFFFFFFFFFFFFFFFFFF ça marche" true true "(R=1.000000,G=0.077258,B=0.000000,A=1.000000)")
  (Variables|Default|SetIsSelected true)
  (bind _asvrpawn_ha_s (Utilities|Casting|CastToVRPawn_HaS (Game|Player|GetPlayerPawn 0)))
  (Variables|/Game/VRMode/Blueprints/VRCamera/VRPawn_HaS.VRPawn_HaS_C|SetSelectedPainting17_0 _asvrpawn_ha_s self)
  (Variables|/Game/VRMode/Blueprints/VRCamera/VRPawn_HaS.VRPawn_HaS_C|SetHasSelectedPainting _asvrpawn_ha_s true)
  (bind _outactors (Actor|GetAllActorsOfClass "/Game/VRMode/Blueprints/Assets/Cadre.Cadre_C"))
  (for _array_element _outactors
    (if (not (== (Variables|/Game/VRMode/Blueprints/Assets/Cadre.Cadre_C|GetCadre_ID _array_element) (Variables|Default|GetCadre_ID)))
      (Rendering|SetActorHiddenInGame _array_element false))))

(event EventOnUpdateTimers
  (params (InteractionTime :type Timer%20Handle%20Structure) (Time :type Float%20%28single-precision%29))
  ;[1 1 1] Interface events
  (Variables|Default|SetInteraction%20Time InteractionTime)
  (Variables|Default|SetTime Time))

(event EventOnDeselect
  (params (CadreID :type Integer))
  (Utilities|FlowControl|Delay 2.0)
  (Variables|Default|SetCadre%20ID%20selected CadreID)
  (Variables|Default|SetIsSelected false)
  (bind _asvrpawn_ha_s (Utilities|Casting|CastToVRPawn_HaS (Game|Player|GetPlayerPawn 0))
    (:then
      (Variables|/Game/VRMode/Blueprints/VRCamera/VRPawn_HaS.VRPawn_HaS_C|SetHasSelectedPainting _asvrpawn_ha_s false)
      (bind _outactors (Actor|GetAllActorsOfClass "/Game/VRMode/Blueprints/Assets/Cadre.Cadre_C"))
      (for _array_element _outactors
        (Rendering|SetActorHiddenInGame _array_element true)
        (if (== (Variables|Default|GetCadre%20ID%20selected) (Variables|/Game/VRMode/Blueprints/Assets/Cadre.Cadre_C|GetCadre_ID _array_element))
          (Variables|Default|SetNewCadreLocation (Transformation|GetActorLocation _array_element)))
        (if (== (Variables|Default|GetCadre_ID) (Variables|/Game/VRMode/Blueprints/Assets/Cadre.Cadre_C|GetCadre_ID _array_element))
          (Variables|Default|SetOldCadreLocation (Transformation|GetActorLocation _array_element))))
      (bind _outactors_2 (Actor|GetAllActorsOfClass "Painting_C"))
      (for _array_element_2 _outactors_2
        (if (== (Variables|Default|GetCadre%20ID%20selected) (Variables|Painting_C|GetCadre_ID _array_element_2))
          (Transformation|SetActorLocation _array_element_2 (Variables|Default|GetOldCadreLocation) false false)
          (Variables|Painting_C|SetCadre_ID _array_element_2 (Variables|Default|GetCadre_ID))))
      (Transformation|SetActorLocation (Variables|Default|GetNewCadreLocation) false false)
      (Variables|Default|SetCadre_ID (Variables|Default|GetCadre%20ID%20selected)))
    (:CastFailed
      (Development|PrintString "cast failed"))))

(event EventBeginPlay
  (bind _outactors (Actor|GetAllActorsOfClass "/Game/VRMode/Blueprints/Assets/Cadre.Cadre_C"))
  (Variables|Default|SetCadres _outactors)
  (bind _outactors_2 (Actor|GetAllActorsOfClass "Painting_C"))
  (Variables|Default|SetPaintings _outactors_2))

(fn ConstructionScript)

(fn GetFocusTime
  (return (Variables|Default|GetFocus%20Time)))
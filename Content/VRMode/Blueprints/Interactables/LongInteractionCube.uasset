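; LongInteractionCube is a VR interactable cube for timed focus interactions, showing progress on a circle widget.
; Interface events receive the timer handle and time, report the focus time, and clear the timer and reset time on blur.
; Every tick it turns the widget toward the player camera and copies the timer and time into it.
; Activation, focus and blur only print debug messages, apart from the blur reset.
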(event EventOnBlur
  ;[1 1 1] Interface events
  (Development|PrintString "BLUR" true true "(R=0.218356,G=1.000000,B=0.000000,A=1.000000)")
  (Utilities|Time|ClearandInvalidateTimerbyHandle (Variables|Default|GetInteraction%20Time))
  (Variables|Default|SetTime 0.0))

(event EventOnFocus
  ;[1 1 1] Interface events
  (Development|PrintString "Focus"))

(event EventTick
  (params (DeltaSeconds :type Float%20%28single-precision%29))
  ;[1 1 1] Draw Circle logic
  (Transformation|SetWorldRotation (Variables|Default|GetCircleWidget) (Math|Rotator|FindLookatRotation (Transformation|GetWorldLocation (Variables|Default|GetCircleWidget)) (Transformation|GetWorldLocation (Variables|/Script/Engine.PlayerCameraManager|GetTransformComponent (Game|GetPlayerCameraManager 0)))) false false)
  (bind _ascircle_widget (Utilities|Casting|CastToCircleWidget (UserInterface|GetWidget (Variables|Default|GetCircleWidget))))
  (Variables|/Game/VRMode/Blueprints/Widgets/InteractionWidgets/CircleWidget.CircleWidget_C|SetTime _ascircle_widget (Variables|Default|GetTime))
  (Variables|/Game/VRMode/Blueprints/Widgets/InteractionWidgets/CircleWidget.CircleWidget_C|SetTimer _ascircle_widget (Variables|Default|GetInteraction%20Time)))

(event EventOnActivate
  ;[1 1 1] Interface events
  (Development|PrintString "WTFFFFFFFFFFFFFFFFFFFFFFFFFFFFFFFFFFFFF ça marche" true true "(R=1.000000,G=0.077258,B=0.000000,A=1.000000)"))

(event EventOnUpdateTimers
  (params (InteractionTime :type Timer%20Handle%20Structure) (Time :type Float%20%28single-precision%29))
  ;[1 1 1] Interface events
  (Variables|Default|SetInteraction%20Time InteractionTime)
  (Variables|Default|SetTime Time))

(fn ConstructionScript)

(fn GetFocusTime
  (return (Variables|Default|GetFocus%20Time)))